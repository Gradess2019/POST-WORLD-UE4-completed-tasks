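; Encyclopedia component that holds the list of encyclopedia entries and tracks which ones have been opened.
; On BeginPlay it copies every row of the encyclopedia data table into the EncyclopediaObjects array.
; OnObjectIsOpened finds entries by name and, if unopened, marks the struct opened and writes it back into the runtime array.
; It prints debug messages and returns true even when no entry matches.
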(event `self.ReceiveBeginPlay`
  ;[1 1 1] Заполняем массив EncyclopediaObjects
  (bind _outrownames (`DataTableFunctionLibrary.GetDataTableRowNames` "/Game/EncyclopediaSystem/DataTable_encyclopediaObjects.DataTable_encyclopediaObjects"))
  (for _array_element _outrownames
    (bind _returnvalue (`|GetDataTableRow` "/Game/EncyclopediaSystem/DataTable_encyclopediaObjects.DataTable_encyclopediaObjects" _array_element)
      (:`then`
        (`KismetArrayLibrary.Array_Add` (`self.encyclopediaObjects`) _returnvalue)))))

(fn `OnObjectIsOpened`
  (params (NameExemplar :type Name))
  (returns (LoopCompleted :type Boolean))
  (for (_array_element _array_index) (`self.encyclopediaObjects`)
    (bind (_name _encyclopediaobjecttype _encyclopediaobjectcategory _isopened _largeimage _icon _descriptionexemplar) (break `/Game/EncyclopediaSystem/Struct_EncyclopediaObjectInfo` _array_element))
    ;[1 1 1] Проверяем, был ли открыт экземпляр ранее. Если нет - устанавливаем значение переменной IsOpen на True и заменяем старое значение в массиве EncyclopediaObjects на новое.
    (if (== NameExemplar _name)
      (if _isopened
        (`KismetSystemLibrary.PrintString` "Exemplar already open" true true (struct :`R` 1.0 :`G` 0.972075 :`A` 1.0))
        (else
          (bind _structout (setmembers `/Game/EncyclopediaSystem/Struct_EncyclopediaObjectInfo` :`StructRef` (make `/Game/EncyclopediaSystem/Struct_EncyclopediaObjectInfo` _name _encyclopediaobjecttype _encyclopediaobjectcategory (`self.IsOpenedSetTrue`) _largeimage _icon _descriptionexemplar)))
          (`KismetArrayLibrary.Array_Set` (`self.encyclopediaObjects`) _array_index _structout)
          (`KismetSystemLibrary.PrintString` "Exemplar Open!" true true (struct :`R` 0.034841 :`G` 1.0 :`B` 0.113513 :`A` 1.0))
          (break)))))
  (`KismetSystemLibrary.PrintString` "Loop Completed")
  (return true))